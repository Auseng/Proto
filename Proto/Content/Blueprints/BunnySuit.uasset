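; BunnySuit is a power-up pickup that temporarily boosts the player's jump.
; On overlap with ProtoPlayer it destroys its Sphere and Collision components, raises player 0's JumpZVelocity, then restores a hard-coded value after a ten-second Delay and destroys itself.
; While idle, Tick rotates the actor by a fixed per-frame step and plays the Movement timeline, which adds local offsets.
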(event Collision|EventActorBeginOverlap
  (params (OtherActor :type Actor%20Object%20Reference))
  (bind _returnvalue (Game|GetPlayerCharacter 0))
  (bind _charactermovement (Variables|/Script/Engine.Character|GetCharacterMovement _returnvalue))
  ;[1 1 1] Bunny Suit
  (Utilities|Casting|CastToProtoPlayer OtherActor)
  (Components|DestroyComponent (Variables|Default|GetSphere))
  (Components|DestroyComponent (Variables|Default|GetCollision))
  (Development|PrintString "Put on Bunny Suit")
  (Variables|/Script/Engine.CharacterMovementComponent|SetJumpZVelocity _charactermovement 8e+02)
  (Utilities|FlowControl|Delay 1e+01)
  (Variables|/Script/Engine.CharacterMovementComponent|SetJumpZVelocity _charactermovement 6e+02)
  (Development|PrintString "Took off Bunny Suit")
  (Actor|DestroyActor))

(event EventTick
  (params (DeltaSeconds :type Float%20%28single-precision%29))
  ;[1 1 1] Power up idle
  (Transformation|AddActorLocalRotation "0,1.000000, 0" false false)
  (bind _movement (Timeline|Movement Play)
    (:Update
      (Transformation|AddActorLocalOffset _movement false false))))

(fn ConstructionScript)