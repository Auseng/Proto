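; Sewing kit health pickup that restores a fixed amount of health to BP_ProtoPlayer on overlap, then destroys itself.
; Any overlap removes its sphere and collision components and prints a message before the player cast, and the health gain is not clamped.
; While idle, Tick spins the actor and plays a timeline that applies movement as local offsets.
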(event Collision|EventActorBeginOverlap
  (params (OtherActor :type Actor%20Object%20Reference))
  ;[1 1 1] Sewing Kit Heal
  (Components|DestroyComponent (Variables|Default|GetSphere2))
  (Components|DestroyComponent (Variables|Default|GetCollision2))
  (Development|PrintString "Use Sewing Kit")
  (bind _asbp_proto_player (Utilities|Casting|CastToBP_ProtoPlayer OtherActor))
  (Variables|/Game/Blueprints/BP_ProtoPlayer.BP_ProtoPlayer_C|SetCurrentHealth _asbp_proto_player (+ (Variables|/Game/Blueprints/BP_ProtoPlayer.BP_ProtoPlayer_C|GetCurrentHealth _asbp_proto_player) 5e+01))
  (Actor|DestroyActor))

(event EventTick
  (params (DeltaSeconds :type Float%20%28single-precision%29))
  ;[1 1 1] Power up idle
  (Transformation|AddActorLocalRotation "0,1.000000, 0" false false)
  (bind _movement (Timeline|Timeline_0 Play)
    (:Update
      (Transformation|AddActorLocalOffset _movement false false))))

(fn ConstructionScript)